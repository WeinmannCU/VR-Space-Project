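; Grabbable bot actor with an animated PanicBot that plays at a slowed rate, freezes while held and resumes when dropped.
; GrabComponent's grab and drop events drive the animation rate.
; On drop, a vertical Visibility trace from above to below the actor snaps it to the impact point and levels it upright, keeping only yaw.
; The trace result is used without checking for a hit.
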(event `self.ReceiveBeginPlay`
  (set `SkeletalMeshComponent.GlobalAnimRateScale` 0.2 (`self.panic_bot`))
  (set `self.player_placed` false))

(event `self.GrabComponent.OnGrabbed`
  (set `SkeletalMeshComponent.GlobalAnimRateScale` 0.0 (`self.panic_bot`)))

(event `self.GrabComponent.OnDropped`
  (set `SkeletalMeshComponent.GlobalAnimRateScale` 0.2 (`self.panic_bot`))
  (bind _output_get (set `self.player_loc` (`self.K2_GetActorLocation`)))
  (bind _outhit (`KismetSystemLibrary.LineTraceSingle` (+ _output_get (0.0 0.0 1000.0)) (- (`self.player_loc`) (`KismetMathLibrary.MakeVector` 0.0 0.0 500.0)) "TraceTypeQuery1"))
  (`self.K2_SetActorLocationAndRotation` (`.ImpactPoint` (`GameplayStatics.BreakHitResult` _outhit)) (`KismetMathLibrary.MakeRotator` 0.0 0.0 (.yaw (`self.K2_GetActorRotation`)))))

(fn `UserConstructionScript`)